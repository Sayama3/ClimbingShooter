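; Enemy AI character with a rifle, a camera-facing health bar and a ragdoll death when health runs out.
; It wanders to random reachable points, while perception moves it toward a sensed player or runs a widening, limited search on other updates.
; Chase moves to a destination, then calls Fire, a rate-limited line-trace shot with montage, effects and damage.
; Perception only prints attack and patrol states, without calling Chase or Fire.
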(event OnTargetPerceptionInfoUpdated(AIPerception)
  (params (UpdateInfo :type Actor%20Perception%20Update%20Info%20Structure%20%28by%20ref%29))
  ;[1 1 1] Comment
  (if (and (== (.target UpdateInfo) (Game|GetPlayerCharacter 0)) (.bsuccessfullysensed (.stimulus UpdateInfo)))
    (Variables|Default|SetHasSeenTarget true)
    (if (<= (Transformation|GetDistanceTo (.target UpdateInfo)) (Variables|Default|GetDistanceShootPlayer))
      (Development|PrintString "Can Attack" :!label _label)
      (else
        (AI|AIMoveTo self (.stimuluslocation (.stimulus UpdateInfo)) 0 (Variables|Default|GetDistanceShootPlayer) false
          (:then
            (Variables|Default|SetIsMoving true))
          (:OnSuccess
            (Variables|Default|SetIsMoving false :!label _label_2)
            (Development|PrintString "Restart the loop"))
          (:OnFail
            (goto _label_2)))))
    (else
      (Variables|Default|SetHasSeenTarget false)
      (AI|AIMoveTo self (.RandomLocation (AI|Navigation|GetRandomReachablePointinRadius (.stimuluslocation (.stimulus UpdateInfo)) (Variables|Default|GetSearchRadius) 0 0)) 0 (Variables|Default|GetDistanceShootPlayer) false :!label _label_3
        (:OnSuccess
          _)
        (:OnFail
          _))
      (if (Variables|Default|GetHasSeenTarget)
        (goto _label)
        (else
          (if (< (Variables|Default|GetNbSeekPlayer) (Variables|Default|GetNbSeekPlayerMax))
            (Variables|Default|SetSearchRadius (* (Variables|Default|GetSearchRadius) 2.0))
            (bind _result (Math|Integer|IncrementInt (Variables|Default|GetNbSeekPlayer))
              (:%20%20
                (if (>= _result (Variables|Default|GetNbSeekPlayerMax))
                  _
                  (else
                    (Development|PrintString "SeekingPlayer")
                    (goto _label_3))))))
          (Variables|Default|SetSearchRadius (/ (Variables|Default|GetSearchRadius) (* (Variables|Default|GetNbSeekPlayer) 2)))
          (Variables|Default|SetNbSeekPlayer 0)
          (Development|PrintString "Patrol"))))))

(event Custom|Search%20Around
  ;[1 1 1] Seach Around
  (if (not (Variables|Default|GetHasSeenTarget))
    (AI|AIMoveTo self (.RandomLocation (AI|Navigation|GetRandomReachablePointinRadius (Transformation|GetActorLocation) (Variables|Default|GetSearchRadius) 0 0)) 0 3e+02 false
      (:OnSuccess
        _)
      (:OnFail
        _))
    (CallFunction|SearchAround)))

(event Custom|Chase
  (params (ChasingPawn :type Pawn%20Object%20Reference) (Destination :type Vector))
  ;[1 1 1] Chase Pawn
  (AI|AIMoveTo self Destination 0 (Variables|Default|GetDistanceShootPlayer) false
    (:OnSuccess
      (CallFunction|Fire Destination))
    (:OnFail
      _))
  (CallFunction|SearchAround))

(event Custom|Fire
  (params (Target :type Vector))
  (bind _sk_rifle (Variables|Default|GetSK_Rifle))
  (bind _returnvalue (Transformation|GetSocketTransform _sk_rifle "b_gun_muzzleflash" "RTS_World"))
  ;[1 1 1] Shoot Pawn
  (if (not (Variables|Default|GetIsDead))
    (Pawn|SetControlRotation (Pawn|GetController) (Math|Rotator|FindLookatRotation (Transformation|GetActorLocation) Target))
    (Utilities|FlowControl|DoOnce false :!label _label
      (:Completed
        (Audio|PlaySoundatLocation "/Game/Sounds/MS_Rifle.MS_Rifle" "0, 0, 0" "0, 0, 0" 1.0 1.0 0.0 0 0 0 0)
        (Effects|SpawnEmitterAttached "/Game/InfinityBladeEffects/Effects/FX_Monsters/FX_Monster_Gruntling/Master/P_BackPack_MuzzleFlash.P_BackPack_MuzzleFlash" _sk_rifle "b_gun_muzzleflash" (.location _returnvalue) (Math|Rotator|MakeRotfromX (Math|Vector|GetUpVector (.rotation _returnvalue))) "0.200000,0.200000,0.200000" "KeepWorldPosition" true "AutoRelease")
        (Animation|Montage|PlayMontage (Variables|Character|GetMesh) (select (Utilities|IsReallyAiming) "/Game/ShooterAnimations/AnimSequence/UE5_Fire_Rifle_Ironsights_Montage.UE5_Fire_Rifle_Ironsights_Montage" "/Game/ShooterAnimations/AnimSequence/UE5_Fire_Rifle_Hip_Montage.UE5_Fire_Rifle_Hip_Montage")
          (:then
            (bind (_returnvalue_2 _outhit) (Utilities|Shoot))
            (if _returnvalue_2
              (Game|Damage|ApplyDamage (.HitActor (Collision|BreakHitResult _outhit)) (Variables|Default|GetWeaponDamage) 0 0)
              (Audio|PlaySoundatLocation "/Game/Sounds/MS_Hit.MS_Hit" (.Location (Collision|BreakHitResult _outhit)) "0, 0, 0" 0.8 1.0 0.0 0 0 0 0)
              (Effects|SpawnEmitteratLocation "/Game/InfinityBladeEffects/Effects/FX_Monsters/FX_Monster_Troll/death/P_TrollDeathImpact.P_TrollDeathImpact" (.Location (Collision|BreakHitResult _outhit)) (Math|Rotator|MakeRotfromX (.Normal (Collision|BreakHitResult _outhit))) "0.800000,0.800000,0.800000" true "AutoRelease"))
            (Utilities|FlowControl|Delay (Variables|Default|GetFireRate))
            (goto _label Reset)))))))

(event EventBeginPlay
  ;[1 1 1] Begin
  (CallFunction|SearchAround))

(event Game|Damage|EventAnyDamage
  (params (Damage :type Float%20%28single-precision%29) (DamageType :type Damage%20Type%20Object%20Reference) (InstigatedBy :type Controller%20Object%20Reference) (DamageCauser :type Actor%20Object%20Reference))
  ;[1 1 1] Health
  (bind _output_get (Variables|Default|SetHealth (- (Variables|Default|GetHealth) Damage)))
  (if (not (> _output_get 0.0))
    (Physics|SetSimulatePhysics (Variables|Character|GetMesh) true)
    (Pawn|Components|CharacterMovement|SetMovementMode (Variables|Character|GetCharacterMovement) "MOVE_None" 0)
    (Rendering|SetVisibility (Variables|Default|GetHealthBarWidget) false false)
    (Variables|Default|SetIsDead true)))

(event EventTick
  (params (DeltaSeconds :type Float%20%28single-precision%29))
  (bind _healthbarwidget (Variables|Default|GetHealthBarWidget))
  (Utilities|FlowControl|Sequence
    (:then_0
      ;[1 1 1] Update UI
      (bind _aswb_ai_health_bar (Utilities|Casting|CastToWB_AI_HEALTH_BAR (UserInterface|GetWidget (Variables|Default|GetHealthBarWidget))))
      (Progress|SetPercent (Variables|/Game/Blueprints/WB_AI_HEALTH_BAR.WB_AI_HEALTH_BAR_C|GetHealthBar _aswb_ai_health_bar) (/ (Variables|Default|GetHealth) 1e+02))
      (Transformation|SetWorldRotation _healthbarwidget (Math|Rotator|FindLookatRotation (Transformation|GetWorldLocation _healthbarwidget) (Camera|GetCameraLocation (Game|GetPlayerCameraManager 0))) false false))))

(fn ConstructionScript)

(fn RotatetoPlayer
  (if (Variables|Default|GetHasSeenTarget)
    (Transformation|SetActorRotation (Math|Rotator|FindLookatRotation (Transformation|GetActorLocation) (Transformation|GetActorLocation (Game|GetPlayerCharacter 0))))
    (else
      (Utilities|Time|ClearTimerbyFunctionName 0 "RotateToPlayer"))))